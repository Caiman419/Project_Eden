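; BP_AmmoBox is an interactable ammo pickup that refills the player's carried ammo.
; On BeginPlay it caches the first player pawn.
; Its Interaction override calls the parent, casts that pawn to NeoEden_MainCharacter, adds its Ammo to PossesedAmmo, refreshes the character's GameHUD and destroys itself.
; Overlap and Tick events are disabled, so the pickup acts only when Interaction is called.
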(event EventBeginPlay
  (|CallParentFunction)
  (Variables|Default|SetPlayer (Game|Player|GetPlayerPawn 0)))

(event Collision|EventActorBeginOverlap
  (params (OtherActor :type Actor%20Object%20Reference))
  (|CallParentFunction OtherActor) ; 지금 이 노드는 비활성 상태입니다. \n핀을 끌어서 다른 노드를 연결하면 활성화됩니다.
)

(event EventTick
  (params (DeltaSeconds :type Float%20%28single-precision%29))
  (|CallParentFunction DeltaSeconds) ; 지금 이 노드는 비활성 상태입니다. \n핀을 끌어서 다른 노드를 연결하면 활성화됩니다.
)

(fn ConstructionScript
  (|CallParentFunction))

(fn Interaction
  (|CallParentFunction)
  (bind _asneo_eden_main_character (Utilities|Casting|CastToNeoEden_MainCharacter (Variables|Default|GetPlayer)))
  (Variables|/Game/Character/NeoEden_MainCharacter.NeoEden_MainCharacter_C|SetPossesedAmmo _asneo_eden_main_character (+ (Variables|/Game/Character/NeoEden_MainCharacter.NeoEden_MainCharacter_C|GetPossesedAmmo _asneo_eden_main_character) (Variables|Default|GetAmmo)))
  (Default|UpdateAmmo (Variables|/Game/Character/NeoEden_MainCharacter.NeoEden_MainCharacter_C|GetGameHUD _asneo_eden_main_character))
  (Actor|DestroyActor))