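; Player component that tracks stamina, handling spending and delayed regeneration.
; UseStamina subtracts a cost, rolls back any spend that would empty stamina, otherwise starts regeneration, and returns whether the resulting stamina is at or below zero.
; A retriggerable delay postpones regeneration until spending pauses, then sets a looping timer whose callback adds one clamped increment and clears that timer on its first tick.
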(event Custom|StartRegenStamina
  ;[0 0 0] Regeneration Stamina
  (Utilities|FlowControl|RetriggerableDelay (Variables|Stamina|GetRegenLatency))
  (bind _returnvalue (Utilities|Time|SetTimerbyEvent (delegate Custom|RegenStamina) 0.1 true))
  (Variables|Timer|SetRegenTimer _returnvalue))

(event Custom|RegenStamina
  ;[0 0 0] Regeneration Stamina
  (Variables|Stamina|SetCurStamina (Math|Float|Clamp(Float) (+ (Variables|Stamina|GetCurStamina) (Variables|Stamina|GetRegenAmount)) 0.0 (Variables|Stamina|GetMaxStamina)))
  (Utilities|Time|ClearandInvalidateTimerbyHandle (Variables|Timer|GetRegenTimer)))

(event EventBeginPlay
  (Variables|GameMode|SetGamemode (Game|GetGameMode)))

(event EventTick
  (params (DeltaSeconds :type Float%20%28single-precision%29)))

(fn UseStamina
  (params (amount :type Float%20%28single-precision%29))
  (Variables|Stamina|Settemp (Variables|Stamina|GetCurStamina))
  (Variables|Stamina|SetCurStamina (Math|Float|Clamp(Float) (- (Variables|Stamina|GetCurStamina) amount) 0.0 (Variables|Stamina|GetCurStamina)))
  (if (<= (Variables|Stamina|GetCurStamina) 0.0)
    (Variables|Stamina|SetCurStamina (Variables|Stamina|Gettemp))
    (else
      (CallFunction|StartRegenStamina)))
  (return (<= (Variables|Stamina|GetCurStamina) 0.0)))