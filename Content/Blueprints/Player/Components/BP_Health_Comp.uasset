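; Player health component that tracks HP, applies damage and regenerates health over time.
; Initialize sets max HP and regen settings, and Damage clamps HP and restarts regeneration through a retriggerable delay and looping one-second timer.
; At zero HP a DoOnce gate clears the regen timer, and RestoreHP refills health, resets that gate and clears the timer.
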(event Custom|Initialize
  (params (MaxHP :type Float%20%28single-precision%29) (RegenAmount :type Float%20%28single-precision%29) (RegenLatency :type Float%20%28single-precision%29))
  (bind _output_get (Variables|HP|SetMaxHP MaxHP))
  (Variables|HP|SetHP _output_get)
  (Variables|HP|SetRegenAmount RegenAmount)
  (Variables|HP|SetRegenLatency RegenLatency))

(event Custom|Damage
  (params (damage :type Float%20%28single-precision%29) (damageCauser :type Actor%20Object%20Reference))
  (Variables|HP|SetHP (Math|Float|Clamp(Float) (- (Variables|HP|GetHP) damage) 0.0 (Variables|HP|GetHP)))
  (if (<= (Variables|HP|GetHP) 0.0)
    (Utilities|FlowControl|DoOnce false
      (:Completed
        (Utilities|Time|ClearandInvalidateTimerbyHandle (Variables|Timer|GetRegenTimer))))
    (else
      (if (Class|KismetSystemLibrary|TimerExistsHandle (Variables|Timer|GetRegenTimer))
        (Utilities|Time|ClearandInvalidateTimerbyHandle (Variables|Timer|GetRegenTimer)))
      (CallFunction|StartRegenHP))))

(event Custom|StartRegenHP
  ;[0 0 0] Regeneration HP
  (Utilities|FlowControl|RetriggerableDelay (Variables|HP|GetRegenLatency))
  (bind _returnvalue (Utilities|Time|SetTimerbyEvent (delegate Custom|RegenHP) 1.0 true))
  (Variables|Timer|SetRegenTimer _returnvalue))

(event Custom|RegenHP
  ;[0 0 0] Regeneration HP
  (Variables|HP|SetHP (Math|Float|Clamp(Float) (+ (Variables|HP|GetHP) (Variables|HP|GetRegenAmount)) 0.0 (Variables|HP|GetMaxHP)))
  (if (not (<= (Variables|HP|GetHP) (Variables|HP|GetMaxHP)))
    (Utilities|Time|ClearandInvalidateTimerbyHandle (Variables|Timer|GetRegenTimer))))

(event Custom|ResetDeathEvent
  (Utilities|FlowControl|DoOnce false) ; enters at Reset
)

(event Custom|RestoreHP
  (Variables|HP|SetHP (Variables|HP|GetMaxHP))
  (CallFunction|ResetDeathEvent)
  (Utilities|Time|ClearandInvalidateTimerbyHandle (Variables|Timer|GetRegenTimer)))

(event EventBeginPlay
  ;[0 0 0] character varible
  (Variables|GameMode|SetGamemode (Game|GetGameMode)))

(event EventTick
  (params (DeltaSeconds :type Float%20%28single-precision%29))
  (if (> 1e+02 (Variables|HP|GetHP))
    _))