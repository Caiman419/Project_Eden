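; BP_Enemy is an enemy Blueprint that tracks a clamped Aggression value; its event graph and Attack function are empty.
; AggressionUp adds aggression and stores its location, recording a timestamp only when exceeding MaxAggro; the ActorAggro input is unused.
; ResetTimer starts a looping one-second timer calling AggressionDown, which lowers aggression by DownAggro scaled by frame delta, floored near zero.
; StopTimer clears that timer; nothing here calls either timer function.
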(event EventBeginPlay)

(event EventTick
  (params (DeltaSeconds :type Float%20%28single-precision%29)))

(fn ConstructionScript)

(fn AggressionUp
  (params (ActorAggro :type BP%20Player%20Object%20Reference) (IncreaseAggro :type Float%20%28single-precision%29) (AggroLocation :type Vector))
  (Variables|Default|SetLastAggroLocation AggroLocation)
  (Variables|Default|SetAggression (+ IncreaseAggro (Variables|Default|GetAggression)))
  (if (> (Math|Float|Truncate (Variables|Default|GetAggression)) (Variables|Default|GetMaxAggro))
    (Variables|Default|SetAggression (Math|Conversions|ToFloat(Integer) (Variables|Default|GetMaxAggro)))
    (Variables|Default|SetLastAggroTime (Utilities|Time|GetTimeSeconds))))

(fn AggressionDown
  (Variables|Default|SetAggression (- (Variables|Default|GetAggression) (* (Variables|Default|GetDownAggro) (Utilities|Time|GetWorldDeltaSeconds))))
  (if (< (Math|Float|Truncate (Variables|Default|GetAggression)) 0)
    (Variables|Default|SetAggression 0.0)))

(fn ResetTimer
  (Utilities|Time|ClearandInvalidateTimerbyHandle (Variables|Default|GetTimerInfo))
  (bind _returnvalue (Utilities|Time|SetTimerbyFunctionName self "AggressionDown" 1.0 true))
  (Variables|Default|SetTimerInfo _returnvalue))

(fn Attack)

(fn StopTimer
  (Utilities|Time|ClearandInvalidateTimerbyHandle (Variables|Default|GetTimerInfo)))