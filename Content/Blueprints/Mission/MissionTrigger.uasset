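; Mission trigger actor that marks a location with a waypoint widget and, when the main character first enters its box, plays a dialogue sequence.
; The waypoint toggles through marker and mission start/end events and updates its distance to the player every tick.
; The one-time overlap reports the location name to the game mode's mission manager and starts a self-rescheduling timer that steps through parallel text, audio and delay arrays on the character's HUD and sound.
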(event OnComponentBeginOverlap(Box)
  (params (OverlappedComponent :type Primitive%20Component%20Object%20Reference) (OtherActor :type Actor%20Object%20Reference) (OtherComp :type Primitive%20Component%20Object%20Reference) (OtherBodyIndex :type Integer) (bFromSweep :type Boolean) (SweepResult :type Hit%20Result%20Structure%20%28by%20ref%29))
  (bind _asneo_eden_main_character (Utilities|Casting|CastToNeoEden_MainCharacter OtherActor))
  (Variables|Default|SetCharacter _asneo_eden_main_character)
  (Utilities|FlowControl|DoOnce false
    (:Completed
      (Variables|Default|SetArrayLength (Utilities|Array|Length (Variables|Default|GetDialog%20Array)))
      (bind _returnvalue (Utilities|Time|SetTimerbyEvent (delegate Custom|Dialog%20Change) 0.2))
      (Variables|Default|SetMultiDialogTimer _returnvalue)
      (Variables|Default|SetcurIndex 0)
      (bind _asbp_new_eden_game_mode (Utilities|Casting|CastToBP_NewEdenGameMode (Game|GetGameMode)))
      (bind _missionmgr (Default|GetMissionManager _asbp_new_eden_game_mode))
      (Default|EnterLocation _missionmgr (Variables|Default|GetLocationName)))))

(event Custom|Dialog%20Change
  (bind _character (Variables|Default|GetCharacter))
  (bind _curindex (Variables|Default|GetcurIndex))
  (Utilities|FlowControl|Sequence
    (:then_0
      (if (<= (Variables|Default|GetArrayLength) _curindex)
        (Utilities|Time|ClearandInvalidateTimerbyHandle (Variables|Default|GetMultiDialogTimer))
        (else
          (Default|SetDialogTextSmoothly (Variables|/Game/Character/NeoEden_MainCharacter.NeoEden_MainCharacter_C|GetGameHUD _character) (Utilities|Array|Get(acopy) (Variables|Default|GetDialog%20Array) _curindex)))))
    (:then_1
      (if (not (<= (Utilities|Array|Length (Variables|Default|GetAudio%20Source)) (Variables|Default|GetcurIndex)))
        (Default|PlayDialogSound _character (Utilities|Array|Get(acopy) (Variables|Default|GetAudio%20Source) (Variables|Default|GetcurIndex)))))
    (:then_2
      (if (not (<= (Utilities|Array|Length (Variables|Default|GetdelayArray)) (Variables|Default|GetcurIndex)))
        (bind _returnvalue (Utilities|Time|SetTimerbyEvent (delegate Custom|Dialog%20Change) (Utilities|Array|Get(acopy) (Variables|Default|GetdelayArray) (Variables|Default|GetcurIndex))))
        (Variables|Default|SetMultiDialogTimer _returnvalue)
        (Math|Integer|IncrementInt (Variables|Default|GetcurIndex))))))

(event Custom|OnStartMission
  (Default|Active (Variables|Default|GetWayPointRef)))

(event Custom|OnEndMission
  (Default|Deactive (Variables|Default|GetWayPointRef)))

(event Custom|HideMarker
  (Default|Deactive (Variables|Default|GetWayPointRef)))

(event Custom|ShowMarker
  (Default|Active (Variables|Default|GetWayPointRef)))

(event EventBeginPlay
  (bind _asbp_way_point (Utilities|Casting|CastToBP_WayPoint (UserInterface|GetUserWidgetObject (Variables|Default|GetWayPoint))))
  (Variables|Default|SetWayPointRef _asbp_way_point))

(event Collision|EventActorBeginOverlap
  (params (OtherActor :type Actor%20Object%20Reference)))

(event EventTick
  (params (DeltaSeconds :type Float%20%28single-precision%29))
  (bind _dist (Default|GetDist (Variables|Default|GetWayPointRef) (Game|Player|GetPlayerPawn 0) self))
  (Default|Update (Variables|Default|GetWayPointRef) _dist))

(fn ConstructionScript)