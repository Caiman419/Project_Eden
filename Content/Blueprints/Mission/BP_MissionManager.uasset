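; Mission manager that tracks the current mission and advances through a chain of missions.
; LoadTable caches rows from the chapter 1 DataTable, and StartMission selects one by ID and broadcasts the change.
; For location-type missions, it notifies the mapped trigger on start and end, and EnterLocation completes the mission when the target name matches.
; Completion starts NextMission, or clears HasMission and broadcasts when that ID is zero.
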(fn EnterLocation
  (params (EnterLocationName :type String))
  (bind _currentmission (Variables|Default|GetCurrentMission))
  (bind (_missionid _missionname _missionsubtext _missiontype _missiontarget) (Utilities|Struct|BreakMissionTableRow _currentmission))
  (if (Utilities|Enum|Equal(Enum) _missiontype "NewEnumerator0")
    (if (Utilities|Enum|Equal(Enum) EnterLocationName (Utilities|Array|Get(acopy) _missiontarget))
      (CallFunction|CompleteMission))))

(fn GetCurrentMission
  (return (Variables|Default|GetCurrentMission)))

(fn CompleteMission
  (bind _missontrigeermap (Variables|Default|GetMissonTrigeerMap))
  (bind _currentmission (Variables|Default|GetCurrentMission))
  (bind (_missionid _missionname _missionsubtext _missiontype _missiontarget _nextmission) (Utilities|Struct|BreakMissionTableRow _currentmission))
  (bind _output (Utilities|Array|Get(acopy) _missiontarget))
  (bind (_value _returnvalue) (Utilities|Map|Find _missontrigeermap _output))
  (if (Utilities|Enum|Equal(Enum) _missiontype "NewEnumerator0")
    (if _returnvalue
      (Default|OnEndMission _value)))
  (if (== _nextmission 0)
    (Variables|Default|SetbHasMission false)
    (Default|CallOnMissionChange)
    (else
      (CallFunction|StartMission _nextmission))))

(fn LoadTable
  (bind _outrownames (DataTable|GetDataTableRowNames "/Game/Blueprints/Mission/MissionTableChap1.MissionTableChap1"))
  (for _array_element _outrownames
    (bind _returnvalue (Utilities|GetDataTableRow "/Game/Blueprints/Mission/MissionTableChap1.MissionTableChap1" _array_element)
      (:then
        (Utilities|Array|Add (Variables|Default|GetMissionTable) _returnvalue)))))

(fn StartMission
  (params (MissionID :type Integer))
  (Variables|Default|SetbHasMission true)
  (bind _array_element (Utilities|Array|ForEachLoopwithBreak (Variables|Default|GetMissionTable))
    (:LoopBody
      (if (== (.MissionID (Utilities|Struct|BreakMissionTableRow _array_element)) MissionID)
        (bind _output_get (Variables|Default|SetCurrentMission _array_element))
        (Default|CallOnMissionChange)
        (if (Utilities|Enum|Equal(Enum) (.MissionType (Utilities|Struct|BreakMissionTableRow _output_get)) "NewEnumerator0")
          (if (.ReturnValue (Utilities|Map|Find (Variables|Default|GetMissonTrigeerMap) (Utilities|Array|Get(acopy) (.MissionTarget (Utilities|Struct|BreakMissionTableRow _output_get)))))
            (Default|OnStartMission (.Value (Utilities|Map|Find (Variables|Default|GetMissonTrigeerMap) (Utilities|Array|Get(acopy) (.MissionTarget (Utilities|Struct|BreakMissionTableRow _output_get))))))))))))