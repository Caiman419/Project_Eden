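; Human enemy Blueprint with an aggro gauge and a pipe melee weapon.
; The construction script creates a dynamic gauge material on Circle, and Tick feeds it aggression as fill and plays state-driven timelines for its color.
; When killed, it hides the gauge and destroys the capsule.
; Pipe overlap damages the main character, then disables the pipe mesh's overlap flag to prevent repeat hits.
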(event OnComponentBeginOverlap(PipeBoxComponent)
  (params (OverlappedComponent :type Primitive%20Component%20Object%20Reference) (OtherActor :type Actor%20Object%20Reference) (OtherComp :type Primitive%20Component%20Object%20Reference) (OtherBodyIndex :type Integer) (bFromSweep :type Boolean) (SweepResult :type Hit%20Result%20Structure%20%28by%20ref%29))
  (if (Variables|/Script/Engine.PrimitiveComponent|GetbGenerateOverlapEvents (Variables|Default|GetPipeMeshComponent))
    (bind _asneo_eden_main_character (Utilities|Casting|CastToNeoEden_MainCharacter OtherActor))
    (Default|TakeDamage _asneo_eden_main_character (Variables|Default|GetWeaponDamage) self)
    (Variables|/Script/Engine.PrimitiveComponent|SetbGenerateOverlapEvents (Variables|Default|GetPipeMeshComponent) false)))

(event EventBeginPlay)

(event Collision|EventActorBeginOverlap
  (params (OtherActor :type Actor%20Object%20Reference)))

(event EventTick
  (params (DeltaSeconds :type Float%20%28single-precision%29))
  (bind _capsulecomponent (Variables|Default|GetCapsuleComponent))
  (|CallParentFunction DeltaSeconds)
  (bind _returnvalue (Class|Enemy|GetKilled))
  (if _returnvalue
    (Rendering|SetVisibility (Variables|Default|GetCircle) false true)
    (if (Utilities|IsValid _capsulecomponent)
      (Components|DestroyComponent _capsulecomponent))
    (else
      (bind _returnvalue_2 (Class|Enemy|GetAggression))
      (Rendering|Material|SetScalarParameterValue (Variables|Default|GetInstanceMat) "AggroPercent" (* _returnvalue_2 0.02) :!class /Script/Engine.MaterialInstanceDynamic) ; 20210616 어그로 게이지 머티리얼 인스턴스화 by 보원
      (bind _returnvalue_3 (Class|Enemy|GetCurState))
      (switch Utilities|FlowControl|Switch|SwitchonEEnemyState _returnvalue_3
        (:Watch
          ;[1 1 1] 어그로 수치에 따른 색깔 변화 부분
          ; 기본 파랑색에서 경계, 수색, 추적에 따라 노랑, 주황, 빨강으로 바뀜
          ; Play from Start에 연결할 것
          (bind _새_트랙_1 (Timeline|Gaurd Play)
            (:Update
              ;;[1 1 1] 20210616
              ;; 어그로 게이지 머티리얼 인스턴스화
              ;; by 보원
              (Rendering|Material|SetVectorParameterValue (Variables|Default|GetInstanceMat) "AggroColor" (Math|Conversions|ToLinearColor(Vector) _새_트랙_1) :!class /Script/Engine.MaterialInstanceDynamic))))
        (:Search
          (bind _color (Timeline|Search Play)
            (:Update
              (Rendering|Material|SetVectorParameterValue (Variables|Default|GetInstanceMat) "AggroColor" (Math|Conversions|ToLinearColor(Vector) _color) :!class /Script/Engine.MaterialInstanceDynamic))))
        (:Track
          (bind _color_2 (Timeline|Chase Play)
            (:Update
              (Rendering|Material|SetVectorParameterValue (Variables|Default|GetInstanceMat) "AggroColor" (Math|Conversions|ToLinearColor(Vector) _color_2) :!class /Script/Engine.MaterialInstanceDynamic))))
        (:Attack
          (Timeline|Chase Play))
        (:BeAttacked
          (Timeline|Chase Play))))))

(fn ConstructionScript
  ;[1 1 1] 20210616
  ; 어그로 게이지 머티리얼 인스턴스화
  ; by 보원
  (bind _returnvalue (Rendering|Material|CreateDynamicMaterialInstance (Variables|Default|GetCircle) 0 "/Game/Meterial/AggroGauge.AggroGauge" "None" :!class /Script/Engine.PrimitiveComponent))
  (bind _output_get (Variables|Default|SetInstanceMat _returnvalue))
  (Rendering|Material|SetVectorParameterValue _output_get "AggroColor" "(R=1.000000,G=0.750000,B=0.000000,A=1.000000)" :!class /Script/Engine.MaterialInstanceDynamic)
  (Rendering|Material|SetScalarParameterValue _output_get "AggroPercent" 0.0 :!class /Script/Engine.MaterialInstanceDynamic))