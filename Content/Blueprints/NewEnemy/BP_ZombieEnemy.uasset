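; Zombie enemy Blueprint that deals melee damage to the main character with its hand.
; On BeginPlay it removes the pipe mesh and two search point components it does not use.
; A Hand overlap while attacking applies fixed damage to NeoEden_MainCharacter, then turns off the hand's overlap events.
; Tick polls the killed state and destroys the capsule once the zombie is dead.
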(event OnComponentBeginOverlap(Hand)
  (params (OverlappedComponent :type Primitive%20Component%20Object%20Reference) (OtherActor :type Actor%20Object%20Reference) (OtherComp :type Primitive%20Component%20Object%20Reference) (OtherBodyIndex :type Integer) (bFromSweep :type Boolean) (SweepResult :type Hit%20Result%20Structure%20%28by%20ref%29))
  (bind _asneo_eden_main_character (Utilities|Casting|CastToNeoEden_MainCharacter OtherActor))
  (bind _returnvalue (Class|HumanEnemy|GetIsAttacking))
  (if _returnvalue
    (bind _output_get (Variables|Default|SetWeaponDamage 15.0))
    (Default|TakeDamage _asneo_eden_main_character _output_get self)
    (Variables|/Script/Engine.PrimitiveComponent|SetbGenerateOverlapEvents (Variables|Default|GetHand) false)))

(event EventBeginPlay
  (Components|DestroyComponent (Variables|Default|GetPipeMeshComponent))
  (Components|DestroyComponent (Variables|Default|GetSearchPointX))
  (Components|DestroyComponent (Variables|Default|GetSearchPointY)))

(event Collision|EventActorBeginOverlap
  (params (OtherActor :type Actor%20Object%20Reference)))

(event EventTick
  (params (DeltaSeconds :type Float%20%28single-precision%29))
  (bind _capsulecomponent (Variables|Default|GetCapsuleComponent))
  (bind _returnvalue (Class|Enemy|GetKilled))
  (if _returnvalue
    (if (Utilities|IsValid _capsulecomponent)
      (Components|DestroyComponent _capsulecomponent))))

(fn ConstructionScript)