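; Human enemy Blueprint that drives an aggression indicator through Material Parameter Collections.
; Each tick it writes scaled aggression to the Circle_Percent collection, then switches on the enemy's current state.
; Watch, Search and Track play color timelines into Circle_Color, noted as shifting from default blue to yellow, orange and red; Attack and Be Attacked reuse the Chase timeline.
; Both collections are global, so instances write to the same values.
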(event EventBeginPlay)

(event Collision|EventActorBeginOverlap
  (params (OtherActor :type Actor%20Object%20Reference)))

(event EventTick
  (params (DeltaSeconds :type Float%20%28single-precision%29))
  (|CallParentFunction DeltaSeconds)
  (bind _returnvalue (Class|Enemy|GetAggression))
  (Rendering|Material|SetScalarParameterValue "/Game/Meterial/Circle_Percent.Circle_Percent" "Percentage" (* _returnvalue 0.02) :!class /Script/Engine.KismetMaterialLibrary)
  (bind _returnvalue_2 (Class|Enemy|GetCurState))
  (switch Utilities|FlowControl|Switch|SwitchonEEnemyState _returnvalue_2
    (:Watch
      ;[1 1 1] 어그로 수치에 따른 색깔 변화 부분
      ; 기본 파랑색에서 경계, 수색, 추적에 따라 노랑, 주황, 빨강으로 바뀜
      ; Play from Start에 연결할 것
      (bind _새_트랙_1 (Timeline|Gaurd Play)
        (:Update
          (Rendering|Material|SetVectorParameterValue "/Game/Meterial/Circle_Color.Circle_Color" "Color" (Math|Conversions|ToLinearColor(Vector) _새_트랙_1) :!class /Script/Engine.KismetMaterialLibrary))))
    (:Search
      (bind _color (Timeline|Search Play)
        (:Update
          (Rendering|Material|SetVectorParameterValue "/Game/Meterial/Circle_Color.Circle_Color" "Color" (Math|Conversions|ToLinearColor(Vector) _color) :!class /Script/Engine.KismetMaterialLibrary))))
    (:Track
      (bind _color_2 (Timeline|Chase Play)
        (:Update
          (Rendering|Material|SetVectorParameterValue "/Game/Meterial/Circle_Color.Circle_Color" "Color" (Math|Conversions|ToLinearColor(Vector) _color_2) :!class /Script/Engine.KismetMaterialLibrary))))
    (:Attack
      (Timeline|Chase Play))
    (:BeAttacked
      (Timeline|Chase Play))))

(fn ConstructionScript)