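; BP_NewEdenGameMode is a game mode that creates and owns the mission manager for the game.
; On BeginPlay it constructs a BP_MissionManager object, stores it and has it load its table.
; It then finds every MissionTrigger actor in the level and registers each in the manager's trigger map, keyed by LocationName.
; GetMissionManager exposes the stored manager to callers.
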(event EventBeginPlay
  (|CallParentFunction)
  (bind _returnvalue (Game|ConstructObjectfromClass "/Game/Blueprints/Mission/BP_MissionManager.BP_MissionManager_C" self))
  (bind _output_get (Variables|Default|SetMissionManager _returnvalue))
  (Utilities|IsValid _output_get
    (:Is%20Valid
      (Default|LoadTable _output_get)
      (bind _outactors (Actor|GetAllActorsOfClass "/Game/Blueprints/Mission/MissionTrigger.MissionTrigger_C"))
      (for _array_element _outactors
        (Utilities|Map|Add (Variables|/Game/Blueprints/Mission/BP_MissionManager.BP_MissionManager_C|GetMissonTrigeerMap _output_get) (Variables|/Game/Blueprints/Mission/MissionTrigger.MissionTrigger_C|GetLocationName _array_element) _array_element)))))

(event EventTick
  (params (DeltaSeconds :type Float%20%28single-precision%29)))

(fn ConstructionScript)

(fn GetMissionManager
  (return (Variables|Default|GetMissionManager)))